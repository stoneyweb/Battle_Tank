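; BP_Tank is the player-controllable tank, connecting its components and input bindings to aiming and movement logic.
; On BeginPlay it passes the barrel and turret to the TankAiming component and both tracks to TankMovement.
; Aim axes rotate an azimuth gimbal for yaw and the spring arm for pitch.
; Move axes send forward and turn intent to TankMovement, and the Fire action calls TankAiming.
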(event `self.ReceiveBeginPlay`
  (`TankAimingComponent.Initialise` (`self.TankAiming`) (`self.Barrel`) (`self.Turret`))
  (`TankMovementComponent.Initialise` (`self.TankMovement`) (`self.Track left`) (`self.Track right`)))

(event `InputAxis|Aim_Azimuth`
  (params (AxisValue :type "Float (single-precision)"))
  ;[1 1 1] Aiming Input Key Mapping
  (`SceneComponent.K2_AddLocalRotation` (`self.AzimuthGimball`) (`KismetMathLibrary.MakeRotator` 0.0 0.0 AxisValue) false false))

(event `InputAxis|Move Forward`
  (params (AxisValue :type "Float (single-precision)"))
  ;[1 1 1] Movement Input Key Mapping
  (`TankMovementComponent.IntendMoveForward` (`self.TankMovement`) AxisValue))

(event `InputAxis|Move Right`
  (params (AxisValue :type "Float (single-precision)"))
  ;[1 1 1] Movement Input Key Mapping
  (`TankMovementComponent.IntendTurnRight` (`self.TankMovement`) AxisValue))

(event `InputAxis|Aim_Elevation`
  (params (AxisValue :type "Float (single-precision)"))
  ;[1 1 1] Aiming Input Key Mapping
  (`SceneComponent.K2_AddLocalRotation` (`self.SpringArm`) (`KismetMathLibrary.MakeRotator` 0.0 AxisValue) false false))

(event `InputAction|Fire`
  (params (Key :type "Key Structure"))
  ;[1 1 1] Aiming Input Key Mapping
  (:`Pressed`
    (`TankAimingComponent.Fire` (`self.TankAiming`))))

(fn `UserConstructionScript`)